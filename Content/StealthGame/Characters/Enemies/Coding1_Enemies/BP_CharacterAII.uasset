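; Stealth-game enemy character that patrols until it sees the player, then gives chase at a faster walk speed.
; Tick selects chase, waypoint-loop patrol or random-point patrol, each using AIMoveTo, with a CanMove flag gating patrol moves but letting chase interrupt.
; PawnSensing sets PlayerVisible on sighting the player, and a retriggerable delay clears it shortly after sightings stop, with debug barks printed.
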(event `self.ReceiveTick`
  (params (DeltaSeconds :type "Float (single-precision)"))
  (if (`self.bCanMove`)
    (if (`self.bPlayerVisible`)
      (`self.ChasePlayer`)
      (elif (`self.bTargetPointMovement`)
        (if (`self.bInChase`)
          (set `self.bInChase` false)
          (`KismetSystemLibrary.Delay` 3.0))
        (`self.MoveToNextPatrolPoint`)
        (else
          (if (`self.bInChase`)
            (set `self.bInChase` false)
            (`KismetSystemLibrary.Delay` 3.0))
          (`self.PatrolRandom`))))
    (elif (`self.bPlayerVisible`)
      (`self.ChasePlayer`))))

(event `self.PawnSensing.OnSeePawn`
  (params (Pawn :type "Pawn Object Reference"))
  (`|ExecutionSequence`
    (:`then_0`
      (cast `/Game/StealthGame/Core/Characters/PlayerCharacter/BP_ThirdPersonCharacterCustom` Pawn
        (:`then`
          (`KismetSystemLibrary.PrintString` "STOP IN THE NAME OF THE LAW")
          (set `self.bPlayerVisible` true))
        (:`CastFailed`
          (set `self.bPlayerVisible` false))))
    (:`then_1`
      (`KismetSystemLibrary.RetriggerableDelay` 1.0)
      (`KismetSystemLibrary.PrintString` "Must've been the wind...")
      (set `self.bPlayerVisible` false))))

(event `ChasePlayer`
  (set `self.bInChase` true)
  (`self.UpdateWalkSpeed` 600.0)
  (set `self.bCanMove` false)
  (`|AIMoveTo` self (0.0 0.0 0.0) (`GameplayStatics.GetPlayerCharacter` 0) 50.0
    (:`OnSuccess`
      _)
    (:`OnFail`
      _))
  (set `self.bCanMove` true))

(event `PatrolRandom`
  (`self.UpdateWalkSpeed` 200.0)
  (set `self.bCanMove` false)
  (`|AIMoveTo` self (`NavigationSystemV1.K2_GetRandomReachablePointInRadius` (`self.K2_GetActorLocation`) 2000.0 null null) null
    (:`OnSuccess`
      _)
    (:`OnFail`
      _))
  (`KismetSystemLibrary.Delay` 3.0)
  (set `self.bCanMove` true))

(event `MoveToNextPatrolPoint`
  (`self.UpdateWalkSpeed` 200.0)
  (set `self.bCanMove` false)
  (`|AIMoveTo` self (0.0 0.0 0.0) (`|GetArrayItem` (`self.PatrolTargetPoints`) (`self.PatrolTargetPointIndex`))
    (:`OnSuccess`
      (`self.SetNextPatrolPointIndex`))
    (:`OnFail`
      _))
  (`KismetSystemLibrary.Delay` 1.0)
  (set `self.bCanMove` true))

(event `SetNextPatrolPointIndex`
  (set `self.PatrolTargetPointIndex` (mod (+ (`self.PatrolTargetPointIndex`) 1) (`KismetArrayLibrary.Array_Length` (`self.PatrolTargetPoints`)))))

(fn `UpdateWalkSpeed`
  (params (NewWalkSpeed :type "Float (double-precision)"))
  (set `CharacterMovementComponent.MaxWalkSpeed` NewWalkSpeed (`self.CharacterMovement`)))

(fn `UserConstructionScript`)